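; BP_ItemEffect is a base Blueprint for inventory item effects, with every function left as an empty stub, apparently for child effects to override.
; Its hooks cover pickup, drop, equip and unequip, each receiving the Player.
; ApplyEffect also takes an Ability, and GetStatChange is a placeholder query that currently returns nothing.
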(fn `ApplyEffect`
  (params (Player :type "/Game/ThirdPerson/Blueprints/BP_ThirdPersonCharacter Object Reference") (Ability :type "/Game/Abilities/Ability Object Reference"))
  (returns (statChange :type "/Game/Inventory/Blueprints/S_statChange Structure"))
  (return))

(fn `GetStatChange`
  (returns (statChanges :type "Array of /Game/Inventory/Blueprints/S_statChange Structure"))
  (return))

(fn `OnDrop`
  (params (Player :type "/Game/ThirdPerson/Blueprints/BP_ThirdPersonCharacter Object Reference"))
  (returns (statChange :type "/Game/Inventory/Blueprints/S_statChange Structure"))
  (return))

(fn `OnEquip`
  (params (Player :type "/Game/ThirdPerson/Blueprints/BP_ThirdPersonCharacter Object Reference"))
  (returns (statChange :type "/Game/Inventory/Blueprints/S_statChange Structure"))
  (return))

(fn `OnPickUp`
  (params (Player :type "/Game/ThirdPerson/Blueprints/BP_ThirdPersonCharacter Object Reference"))
  (returns (statChange :type "/Game/Inventory/Blueprints/S_statChange Structure"))
  (return))

(fn `OnUnequip`
  (params (Player :type "/Game/ThirdPerson/Blueprints/BP_ThirdPersonCharacter Object Reference"))
  (returns (statChange :type "/Game/Inventory/Blueprints/S_statChange Structure"))
  (return))