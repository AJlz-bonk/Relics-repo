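; Enemy AI Blueprint that stands still until pawn sensing spots a pawn, then chases the player and attacks on arrival.
; FollowPlayer runs AI MoveTo toward the player and, on success, calls AttackFunction behind flag checks and a short delay.
; AttackFunction damages actors overlapping its sphere that lie in front, using a dot-product facing test.
; Incoming damage lowers Health and destroys the actor at zero.
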(event `self.ReceiveAnyDamage`
  (params (Damage :type "Float (single-precision)") (DamageType :type "DamageType Object Reference") (InstigatedBy :type "Controller Object Reference") (DamageCauser :type "Actor Object Reference"))
  (bind _health (`self.Health`))
  (set `self.Health` (- _health Damage))
  (`KismetSystemLibrary.PrintString` (`KismetStringLibrary.Conv_DoubleToString` _health))
  (if (<= _health 0.0)
    (`self.K2_DestroyActor`)
    (`KismetSystemLibrary.PrintString` "I died")))

(event `self.ReceiveTick`
  (params (DeltaSeconds :type "Float (single-precision)"))
  (if (not (`self.IsSeeingPlayeer`))
    (`MovementComponent.StopMovementImmediately` (`self.CharacterMovement`))))

(event `self.PawnSensing.OnSeePawn`
  (params (Pawn :type "Pawn Object Reference"))
  (set `self.IsSeeingPlayeer` true)
  (`self.Follow Player`))

(event `Follow Player`
  (set `self.isAttacking` false)
  (set `self.CanAttack` true)
  (`|AIMoveTo` self (0.0 0.0 0.0) (`GameplayStatics.GetPlayerCharacter` 0)
    (:`OnSuccess`
      (if (`self.CanAttack`)
        (if (not (`self.isAttacking`))
          (set `self.CanAttack` false)
          (`self.AttackFunction`)
          (`KismetSystemLibrary.Delay` 0.2)
          (set `self.isAttacking` false)
          (set `self.CanAttack` true))))))

(fn `AttackFunction`
  (set `self.isAttacking` true)
  (for _array_element (`PrimitiveComponent.GetOverlappingActors` (`self.Sphere`) "/Script/Engine.Actor")
    (if (> (`KismetMathLibrary.Dot_VectorVector` (`KismetMathLibrary.GetDirectionUnitVector` (`self.K2_GetActorLocation`) (`self.K2_GetActorLocation` _array_element)) (`self.GetActorForwardVector`)) 0.0)
      ;[1 1 1] Make sure to change the base damage base don the str stat later
      (`GameplayStatics.ApplyDamage` _array_element 20.0 null (`self.GetOwner`)))))

(fn `UserConstructionScript`)