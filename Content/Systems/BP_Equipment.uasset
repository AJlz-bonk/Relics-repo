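; BP_Equipment holds the player's equipment as a four-slot item array and manages the widget that displays it.
; On BeginPlay it creates WB_Equipment, sizes the array and passes itself to the widget's LoadEquipment.
; The O key toggles the widget in the viewport, and K prints each item's name and type for debugging.
; Nodes for showing the cursor and switching to UI-only input are present but unconnected.
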(event `self.ReceiveBeginPlay`
  (bind _returnvalue (`|CreateWidget` "/Game/UI/InventoryWBs/WB_Equipment.WB_Equipment_C"))
  (set `self.EquipmentInventory` _returnvalue)
  (`KismetArrayLibrary.Array_Resize` (`self.Equipment`) 4)
  (`/Game/UI/InventoryWBs/WB_Equipment.LoadEquipment` (`self.EquipmentInventory`) self))

(event `Key|O`
  (params (Key :type "Key Structure"))
  (bind _equipmentinventory (`self.EquipmentInventory`))
  (:`Pressed`
    (if (`Widget.IsVisible` _equipmentinventory)
      (`Widget.RemoveFromParent` _equipmentinventory)
      (else
        (`UserWidget.AddToViewport` _equipmentinventory 0)))))

(event `Key|K`
  (params (Key :type "Key Structure"))
  (:`Pressed`
    (for _array_element (`self.Equipment`)
      (bind (_name _stackable _stacksize _thumbnail _mesh _itemid _itemtype) (break `/Game/Inventory/Blueprints/ItemStruct` _array_element))
      (`KismetSystemLibrary.PrintString` (`KismetStringLibrary.Concat_StrStr` (`KismetStringLibrary.Concat_StrStr` _name ", ") _itemtype) true true (struct :`R` 1.0 :`B` 0.062022 :`A` 1.0) 5.0))))