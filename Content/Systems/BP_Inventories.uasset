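; Inventory system that builds the inventory UI and lets the player pick up nearby items.
; On BeginPlay it creates the panels widget and three panel managers, one per inventory type.
; Pressing F sphere-traces around the player's lower body, destroying each BP_Item successfully added.
; Adding looks up item details in the GameInstance, fills the first compatible capped stack or empty slot in the first inventory, and reloads that slot.
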(event `self.ReceiveBeginPlay`
  (bind _returnvalue (`|CreateWidget` "/Game/UI/InventoryWBs/WB_InventoryPanels.WB_InventoryPanels_C"))
  (bind _output_get (set `self.inventoryPanels` _returnvalue))
  (`UserWidget.AddToViewport` _output_get 0)
  (bind _panels (`/Game/UI/InventoryWBs/WB_InventoryPanels.GetPanels` _output_get))
  (for _index (range 3)
    (bind _output (`|GetArrayItem` _panels _index))
    (bind _returnvalue_2 (`|CreateWidget` "/Game/Inventory/Blueprints/WB_PanelManager.WB_PanelManager_C" null _index _output (`self.inventoryPanels`)))
    (`/Game/Inventory/Blueprints/WB_PanelManager.Initialize` _returnvalue_2 _output)
    (`KismetArrayLibrary.Array_Set` (`self.inventories`) _index _returnvalue_2)))

(event `Key|F`
  (params (Key :type "Key Structure"))
  (bind _returnvalue (- (`Actor.K2_GetActorLocation` (`GameplayStatics.GetPlayerCharacter` 0)) (0.0 0.0 65.0)))
  (:`Pressed`
    (bind _outhits (`KismetSystemLibrary.SphereTraceMulti` :`Start` _returnvalue :`End` _returnvalue :`Radius` 100.0 :`TraceChannel` "TraceTypeQuery1" :`DrawDebugType` "ForDuration" :`DrawTime` 0.2))
    (for _array_element _outhits
      (bind _asbp_item (cast `/Game/Inventory/Blueprints/BP_Item` (`.HitActor` (`GameplayStatics.BreakHitResult` _array_element))))
      (`/Engine/EditorBlueprintResources/StandardMacros.IsValid` _asbp_item
        (:`Is Valid`
          (bind _succeeded_ (`self.Add Item to Inventory` (`/Game/Inventory/Blueprints/BP_Item.item` _asbp_item)))
          (if _succeeded_
            (`Actor.K2_DestroyActor` _asbp_item)))))))

(fn `Add Item to Inventory`
  (params (Item :type "/Game/Inventory/Blueprints/S_Item Structure"))
  (returns (`Succeeded?` :type Boolean))
  (locals (itemToAdd :type "/Game/Inventory/Blueprints/S_Item Structure") (itemDetailToAdd :type "/Game/Inventory/Blueprints/S_ItemDetail Structure") (arrayIndex :type Integer) (newStackSize :type Integer) (newIndex :type Integer))
  (bind (_id _stacksize) (break `/Game/Inventory/Blueprints/S_Item` (`local.itemToAdd`)))
  (set `local.itemToAdd` Item)
  (bind _asbp_game_instance (cast `/Game/BP_GameInstance` (`GameplayStatics.GetGameInstance`))
    (:`then`
      _)
    (:`CastFailed`
      _))
  (set `local.itemDetailToAdd` (`BlueprintMapLibrary.Map_Find` (`/Game/BP_GameInstance.itemMap` _asbp_game_instance) (`.ID_5_0857C4E24E723564A1427B84C2F76CD9` (break `/Game/Inventory/Blueprints/S_Item` (`local.itemToAdd`)))))
  (for (_array_element _array_index) (`/Game/Inventory/Blueprints/WB_PanelManager.items` (`|GetArrayItem` (`self.inventories`)))
    (set `local.arrayIndex` _array_index)
    (bind (_id_2 _stacksize_2) (break `/Game/Inventory/Blueprints/S_Item` _array_element))
    (bind _output_get (set `local.newStackSize` (+ _stacksize_2 _stacksize)))
    (if (and (<= _output_get 10) (== _id_2 _id) (`.stackable_8_7257542348919A836ED601B2FEA279C5` (break `/Game/Inventory/Blueprints/S_ItemDetail` (`local.itemDetailToAdd`))))
      (`KismetArrayLibrary.Array_Set` (`/Game/Inventory/Blueprints/WB_PanelManager.items` (`|GetArrayItem` (`self.inventories`))) (`local.arrayIndex`) (make `/Game/Inventory/Blueprints/S_Item` (`.ID_5_0857C4E24E723564A1427B84C2F76CD9` (break `/Game/Inventory/Blueprints/S_Item` (`local.itemToAdd`))) (`local.newStackSize`)))
      (bind _box (`/Game/UI/InventoryWBs/WB_PanelBase.GetWrapBox` (`/Game/Inventory/Blueprints/WB_PanelManager.UIPanel` (`|GetArrayItem` (`self.inventories`))) :!label _label))
      (bind _aswb_inventory_slot (cast `/Game/UI/InventoryWBs/WB_inventorySlot` (`PanelWidget.GetChildAt` _box (`local.arrayIndex`))))
      (`/Game/UI/InventoryWBs/WB_inventorySlot.ReloadSlot` _aswb_inventory_slot)
      (return true)
      (elif (== _id_2 0)
        (`KismetArrayLibrary.Array_Set` (`/Game/Inventory/Blueprints/WB_PanelManager.items` (`|GetArrayItem` (`self.inventories`))) (`local.arrayIndex`) (`local.itemToAdd`))
        (goto _label)))))