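; BP_Inventory manages the player's item slots, creating a WBInventory widget that the I key shows or hides.
; Pressing E runs a debug-drawn sphere trace low on the player character to find BP_Item actors.
; Each found item goes into the first slot that is either empty or a matching stackable with room under the fixed cap, then the widget reloads and the world actor is destroyed.
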(event `self.ReceiveBeginPlay`
  (bind _returnvalue (`|CreateWidget` "/Game/UI/HudWBs/WBInventory.WBInventory_C"))
  (set `self.InventoryWidget` _returnvalue)
  (`KismetArrayLibrary.Array_Resize` (`self.Items`) (`self.InventorySize`))
  (`/Game/UI/HudWBs/WBInventory.LoadInventory` (`self.InventoryWidget`) self))

(event `Key|I`
  (params (Key :type "Key Structure"))
  (bind _inventorywidget (`self.InventoryWidget`))
  (:`Pressed`
    (if (`Widget.IsVisible` (`self.InventoryWidget`))
      (`Widget.RemoveFromParent` _inventorywidget)
      (else
        (`UserWidget.AddToViewport` _inventorywidget 0)))))

(event `Key|E`
  (params (Key :type "Key Structure"))
  (bind (_item_name _item_stackable _item_stacksize _item_thumbnail _item_mesh) (break `/Game/Inventory/Blueprints/ItemStruct` (`/Game/Inventory/Blueprints/BP_Item.Item` (`self.itemToPickUp`))))
  (bind _returnvalue (- (`Actor.K2_GetActorLocation` (`GameplayStatics.GetPlayerCharacter` 0)) (0.0 0.0 65.0)))
  (:`Pressed`
    (bind _outhits (`KismetSystemLibrary.SphereTraceMulti` :`Start` _returnvalue :`End` _returnvalue :`Radius` 120.0 :`TraceChannel` "TraceTypeQuery1" :`DrawDebugType` "ForDuration" :`DrawTime` 0.5))
    (for _array_element _outhits
      (bind _asbp_item (cast `/Game/Inventory/Blueprints/BP_Item` (`.HitActor` (`GameplayStatics.BreakHitResult` _array_element))))
      (bind _output_get (set `self.itemToPickUp` _asbp_item))
      (for (_array_element_2 _array_index) (`self.Items`)
        (set `self.Array Index` _array_index)
        (`/Engine/EditorBlueprintResources/StandardMacros.IsValid` (`self.itemToPickUp`)
          (:`Is Valid`
            (bind (_name _stackable _stacksize) (break `/Game/Inventory/Blueprints/ItemStruct` _array_element_2))
            (bind _item (`/Game/Inventory/Blueprints/BP_Item.Item` _output_get))
            (bind (_name_2 _stackable_2 _stacksize_2) (break `/Game/Inventory/Blueprints/ItemStruct` _item))
            (bind _output_get_2 (set `self.NewStackSize` (+ _stacksize _stacksize_2)))
            (if (and (`KismetTextLibrary.EqualEqual_TextText` _name _name_2) (<= _output_get_2 10) _stackable_2)
              (`KismetArrayLibrary.Array_Set` (`self.Items`) (`self.Array Index`) (make `/Game/Inventory/Blueprints/ItemStruct` _item_name _item_stackable (`self.NewStackSize`) _item_thumbnail _item_mesh))
              (`/Game/UI/HudWBs/WBInventory.LoadInventory` (`self.InventoryWidget`) self :!label _label)
              (`Actor.K2_DestroyActor` (`self.itemToPickUp`))
              (elif (== _stacksize 0)
                (`KismetArrayLibrary.Array_Set` (`self.Items`) (`self.Array Index`) _item)
                (goto _label)))))))))