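; BP_Stats is a component that tracks stats, level, health and potential as name-keyed maps.
; RefreshStats rebuilds current stats from base stats, applying additive or multiplicative changes from the player's equipped item effects and temporary buffs.
; Owner damage reduces health percent relative to current max health.
; Tick regenerates potential percent up to full, and ChangePotential reports when it is depleted.
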(event `self.ReceiveBeginPlay`
  (add `Actor.OnTakeAnyDamage` (`self.GetOwner`) (delegate `OnDamaged`))
  (bind _asbp_game_instance (cast `/Game/BP_GameInstance` (`GameplayStatics.GetGameInstance`))
    (:`then`
      _)
    (:`CastFailed`
      _))
  (set `self.itemMap` (`/Game/BP_GameInstance.itemMap` _asbp_game_instance)))

(event `OnDamaged`
  (params (DamagedActor :type "Actor Object Reference") (Damage :type "Float (single-precision)") (DamageType :type "DamageType Object Reference") (InstigatedBy :type "Controller Object Reference") (DamageCauser :type "Actor Object Reference"))
  ;[1 1 1] Converts damage to a %
  (`BlueprintMapLibrary.Map_Add` (`self.baseStats`) "healthPercent" (- (`BlueprintMapLibrary.Map_Find` (`self.baseStats`) "healthPercent") (/ Damage (`BlueprintMapLibrary.Map_Find` (`self.currStats`) "health")))))

(event `self.ReceiveTick`
  (params (DeltaSeconds :type "Float (single-precision)"))
  (if (>= (`BlueprintMapLibrary.Map_Find` (`self.baseStats`) "potentialPercent") 1.0)
    (`BlueprintMapLibrary.Map_Add` (`self.baseStats`) "potentialPercent" 1.0)
    (else
      (`self.changePotential` (* DeltaSeconds -5.0)))))

(fn `addStatChanger`
  (params (statChangeStruct :type "/Game/Inventory/Blueprints/S_statChange Structure"))
  (`KismetArrayLibrary.Array_Add` (`self.statChanges`) statChangeStruct))

(fn `applyStatChanges`
  (locals (statChanger :type "/Game/Inventory/Blueprints/S_statChange Structure"))
  (bind (_ismult _statchanges) (break `/Game/Inventory/Blueprints/S_statChange` (`local.statChanger`)))
  (for _array_element (`self.statChanges`)
    (set `local.statChanger` _array_element)
    (bind _keys (`BlueprintMapLibrary.Map_Keys` (`self.currStats`)))
    (for _array_element_2 _keys
      (bind (_value _returnvalue) (`BlueprintMapLibrary.Map_Find` _statchanges _array_element_2))
      (if _returnvalue
        (if _ismult
          (bind _value_2 (`BlueprintMapLibrary.Map_Find` (`self.currStats`) _array_element_2))
          (`BlueprintMapLibrary.Map_Add` (`self.currStats`) _array_element_2 (* _value_2 _value))
          (else
            (`BlueprintMapLibrary.Map_Add` (`self.currStats`) _array_element_2 (+ _value_2 _value))))))))

(fn `changePotential`
  (params (potentialChange :type "Float (double-precision)"))
  (returns (isNegative :type Boolean))
  (`BlueprintMapLibrary.Map_Add` (`self.baseStats`) "potentialPercent" (- (`BlueprintMapLibrary.Map_Find` (`self.baseStats`) "potentialPercent") (/ potentialChange (`BlueprintMapLibrary.Map_Find` (`self.currStats`) "potential"))))
  (return (<= (`BlueprintMapLibrary.Map_Find` (`self.baseStats`) "potentialPercent") 0.0)))

(fn `getStats`
  (returns (baseStats :type "Map of String to Float (double-precision)") (currStats :type "Map of String to Float (double-precision)"))
  (return (`self.baseStats`) (`self.currStats`)))

(fn `LevelUp`
  (set `self.PlayerLevel` (`KismetMathLibrary.Clamp` (+ (`self.PlayerLevel`) 1) 1 50)))

(fn `QueryStat`
  (params (Stat :type String))
  (returns (Val :type "Float (double-precision)"))
  (return (`BlueprintMapLibrary.Map_Find` (`self.currStats`) Stat)))

(fn `refreshStats`
  (`KismetArrayLibrary.Array_Clear` (`self.statChanges`))
  (bind _asbp_third_person_character (cast `/Game/ThirdPerson/Blueprints/BP_ThirdPersonCharacter` (`GameplayStatics.GetPlayerCharacter` 0)))
  ; Goes through eqp
  (for (_array_element _array_index) (`/Game/Systems/BP_Inventories.inventories` (`/Game/ThirdPerson/Blueprints/BP_ThirdPersonCharacter.Inventories` _asbp_third_person_character))
    (if (== _array_index 1)
      ; Goes through inventory
      (for _array_element_2 (`/Game/Inventory/Blueprints/WB_PanelManager.Items` _array_element)
        (for _array_element_3 (`.Effects_39_4B5A909A45DF9611943C0B93F6F7AA7E` (break `/Game/Inventory/Blueprints/S_ItemDetail` (`BlueprintMapLibrary.Map_Find` (`self.itemMap`) (`.ID_5_0857C4E24E723564A1427B84C2F76CD9` (break `/Game/Inventory/Blueprints/S_Item` _array_element_2)))))
          ; Goes through effects
          (bind _returnvalue (`|GenericCreateObject` _array_element_3))
          (bind _statchanges (`/Game/Inventory/Blueprints/ItemEffects/BP_ItemEffect.GetStatChange` _returnvalue))
          (for _array_element_4 _statchanges
            (`KismetArrayLibrary.Array_Add` (`self.statChanges`) _array_element_4))))))
  (for _array_element_5 (`self.tempBuffs`)
    (`KismetArrayLibrary.Array_Add` (`self.statChanges`) _array_element_5))
  (set `self.currStats` (`self.baseStats`))
  (`self.applyStatChanges`))