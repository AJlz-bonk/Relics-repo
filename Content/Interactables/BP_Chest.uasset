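; Interactable chest that spawns a random loot item in front of itself on each Interact while Uses remain.
; Interact randomly picks relic, rune, armor or weapon, then decrements Uses.
; Each spawn function creates a BP_Item with an ID from its category's range; only relics get random stack sizes, and runes always get ID 7 despite the commented range.
; A sphere overlap toggles a widget for BP_ThirdPersonCharacter.
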(event `self.ReceiveBeginPlay`)

(event `/Game/Systems/InteractInterface.Interact`
  (if (> (`self.uses`) 0)
    (switch `int` (`KismetMathLibrary.RandomInteger` 4)
      (:`0`
        (`self.spawnRelic`))
      (:`1`
        (`self.spawnRune`))
      (:`2`
        (`self.spawnArmor`))
      (:`3`
        (`self.spawnWeapon`)))
    (set `self.uses` (- (`self.uses`) 1))))

(event `self.Sphere.OnComponentBeginOverlap`
  (params (OverlappedComponent :type "PrimitiveComponent Object Reference") (OtherActor :type "Actor Object Reference") (OtherComp :type "PrimitiveComponent Object Reference") (OtherBodyIndex :type Integer) (bFromSweep :type Boolean) (SweepResult :type "HitResult Structure (by ref)"))
  (cast `/Game/ThirdPerson/Blueprints/BP_ThirdPersonCharacter` OtherActor)
  (`SceneComponent.SetVisibility` (`self.Widget`) true false))

(event `self.Sphere.OnComponentEndOverlap`
  (params (OverlappedComponent :type "PrimitiveComponent Object Reference") (OtherActor :type "Actor Object Reference") (OtherComp :type "PrimitiveComponent Object Reference") (OtherBodyIndex :type Integer))
  (cast `/Game/ThirdPerson/Blueprints/BP_ThirdPersonCharacter` OtherActor)
  (`SceneComponent.SetVisibility` (`self.Widget`) false false))

(fn `spawnArmor`
  (`|SpawnActorFromClass` "/Game/Inventory/Blueprints/BP_Item.BP_Item_C" (`KismetMathLibrary.MakeTransform` (+ (* (`self.GetActorForwardVector`) 100.0) (`self.K2_GetActorLocation`)) (`self.K2_GetActorRotation`)) "Undefined" "MultiplyWithRoot" null (make `/Game/Inventory/Blueprints/S_Item` (+ (`KismetMathLibrary.RandomInteger` 2) 10) 1) null))

(fn `spawnRelic`
  (`|SpawnActorFromClass` "/Game/Inventory/Blueprints/BP_Item.BP_Item_C" (`KismetMathLibrary.MakeTransform` (+ (* (`self.GetActorForwardVector`) 100.0) (`self.K2_GetActorLocation`)) (`self.K2_GetActorRotation`)) "Undefined" "MultiplyWithRoot" null (make `/Game/Inventory/Blueprints/S_Item` (+ (`KismetMathLibrary.RandomInteger` 5) 1) (+ (`KismetMathLibrary.RandomInteger` 5) 1)) null))

(fn `spawnRune`
  (`|SpawnActorFromClass` "/Game/Inventory/Blueprints/BP_Item.BP_Item_C" (`KismetMathLibrary.MakeTransform` (+ (* (`self.GetActorForwardVector`) 100.0) (`self.K2_GetActorLocation`)) (`self.K2_GetActorRotation`)) "Undefined" "MultiplyWithRoot" null (make `/Game/Inventory/Blueprints/S_Item` (+ 1 6) 1) null))

(fn `spawnWeapon`
  (`|SpawnActorFromClass` "/Game/Inventory/Blueprints/BP_Item.BP_Item_C" (`KismetMathLibrary.MakeTransform` (+ (* (`self.GetActorForwardVector`) 100.0) (`self.K2_GetActorLocation`)) (`self.K2_GetActorRotation`)) "Undefined" "MultiplyWithRoot" null (make `/Game/Inventory/Blueprints/S_Item` (+ (`KismetMathLibrary.RandomInteger` 2) 12) 1) null))

(fn `UserConstructionScript`)