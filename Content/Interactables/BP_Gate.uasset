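; BP_Gate is a level-transition gate that sends the player into the dungeon.
; When its TriggerBox is overlapped and IsOverlapping is true, it checks that the other actor is a BP_ThirdPersonCharacter.
; It then blocking-loads DungeonLevel as a visible streamed level and teleports the character to a hardcoded location.
; Debug prints trace each step, and the LobbyLevel unload is left disconnected.
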(event `self.TriggerBox.OnComponentBeginOverlap`
  (params (OverlappedComponent :type "PrimitiveComponent Object Reference") (OtherActor :type "Actor Object Reference") (OtherComp :type "PrimitiveComponent Object Reference") (OtherBodyIndex :type Integer) (bFromSweep :type Boolean) (SweepResult :type "HitResult Structure (by ref)"))
  (if (`self.isOverlapping`)
    (if (`KismetSystemLibrary.IsValid` OtherActor)
      (bind _asbp_third_person_character (cast `/Game/ThirdPerson/Blueprints/BP_ThirdPersonCharacter` OtherActor)
        (:`then`
          (`KismetSystemLibrary.PrintString` "cast didn't fail" true true (struct :`G` 0.66 :`B` 1.0 :`A` 1.0) 1000.0)
          ; Comment
          (`GameplayStatics.LoadStreamLevel` "DungeonLevel" true true)
          (`KismetSystemLibrary.PrintString` "New level loaded" true true (struct :`G` 0.66 :`B` 1.0 :`A` 1.0) 1000.0)
          (`self.K2_TeleportTo` :`self` _asbp_third_person_character :`DestLocation` (300.0 300.0 0.0))
          (`KismetSystemLibrary.PrintString` "player teleported" true true (struct :`G` 0.66 :`B` 1.0 :`A` 1.0) 1000.0))
        (:`CastFailed`
          (`KismetSystemLibrary.PrintString` "Cast failed" true true (struct :`G` 0.66 :`B` 1.0 :`A` 1.0) 1000.0))))))

(fn `UserConstructionScript`)